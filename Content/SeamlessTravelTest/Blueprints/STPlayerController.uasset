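; Player controller for a seamless travel test that triggers level travel and owns a loading screen widget.
; On begin play it focuses the game viewport, then creates a Loadscreen_UW widget and adds it to the viewport.
; Pressing T casts the game mode to ThirdPersonGameMode and calls TravelToNextLevel.
; ToggleLoadscreen forwards a value to that widget, or prints a warning if the widget is invalid.
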(event Input|KeyboardEvents|T
  (params (Key :type Key%20Structure :default "None"))
  (:Pressed
    (bind _asthird_person_game_mode (Utilities|Casting|CastToThirdPersonGameMode (Game|GetGameMode)))
    (Default|TraveltoNextLevel _asthird_person_game_mode)))

(fn ConstructionScript)

(fn ReceiveBeginPlay
  (Class|WidgetBlueprintLibrary|SetFocustoGameViewport)
  (bind _returnvalue (UserInterface|CreateWidget "/Game/SeamlessTravelTest/Blueprints/Loadscreen_UW.Loadscreen_UW_C" (Game|GetPlayerController 0)))
  (bind _output_get (Variables|Default|SetLoadscreenWidgetRef _returnvalue))
  (UserInterface|Viewport|AddtoViewport _output_get 0))

(fn ToggleLoadscreen
  (params (Value :type Boolean))
  (Variables|Default|GetLoadscreenWidgetRef
    (:then
      (Default|ToggleLoadscreen (Variables|Default|GetLoadscreenWidgetRef) Value))
    (:else
      (Development|PrintString "Can't toggle loadscreen"))))